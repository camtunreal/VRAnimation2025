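; Cannon Blueprint that plays a one-shot firing sequence automatically on BeginPlay.
; It stores the starting relative rotations of the lever and cannon rotator, then chains two timelines that lerp each to its target as a world rotation, lever first.
; When the cannon finishes rotating, it spawns a scaled-up projectile at the Arrow component's location and rotation.
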(event `self.ReceiveBeginPlay`
  (bind (_returnvalue_location _returnvalue_rotation) (`KismetMathLibrary.BreakTransform` (`SceneComponent.K2_GetComponentToWorld` (`self.Arrow`))))
  (set `self.First Lever Rotation` (`SceneComponent.RelativeRotation` (`self.Lever`)))
  (set `self.First Cannon Rotation` (`SceneComponent.RelativeRotation` (`self.CannonRotator`)))
  (bind (_direction _speed) (`Timeline|Timeline` :!via `PlayFromStart`)
    (:`Update`
      (`SceneComponent.K2_SetWorldRotation` (`self.Lever`) (`KismetMathLibrary.RLerp` (`self.First Lever Rotation`) (`self.Target Lever Rotation`) _speed) false false))
    (:`Finished`
      (bind (_direction_2 _speed_2) (`Timeline|Timeline_0` :!via `PlayFromStart`)
        (:`Update`
          (`SceneComponent.K2_SetWorldRotation` (`self.CannonRotator`) (`KismetMathLibrary.RLerp` (`self.First Cannon Rotation`) (`self.Target Cannon Rotation`) _speed_2) false false))
        (:`Finished`
          (`|SpawnActorFromClass` "/Game/VRTemplate/Blueprints/Projectile.Projectile_C" (`KismetMathLibrary.MakeTransform` _returnvalue_location _returnvalue_rotation (5.0 5.0 5.0)) "Undefined" "MultiplyWithRoot" null null))))))

(fn `UserConstructionScript`)